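; SaveStand is a save station actor with a map stand where the player can save the game.
; Its box overlap sets the ski character's AtSaveStation flag, calls the HUD's EnterPrompt on both entry and exit, and swaps a stand material slot between a map and an invisible material.
; A separate Use event calls SaveFPgame on the player character, without checking the overlap itself.
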(event `self.Box.OnComponentBeginOverlap`
  (params (OverlappedComponent :type "PrimitiveComponent Object Reference") (OtherActor :type "Actor Object Reference") (OtherComp :type "PrimitiveComponent Object Reference") (OtherBodyIndex :type Integer) (bFromSweep :type Boolean) (SweepResult :type "HitResult Structure (by ref)"))
  (bind _asbp_ski_character (cast `/Game/Blueprints/Blueprints/BP_SkiCharacter` OtherActor))
  (set `/Game/Blueprints/Blueprints/BP_SkiCharacter.AtSaveStation` true _asbp_ski_character)
  (`/Game/Blueprints/Blueprints/UI/Hud.EnterPrompt` (`/Game/Blueprints/Blueprints/BP_SkiCharacter.HUD` _asbp_ski_character))
  (`PrimitiveComponent.SetMaterial` (`self.MapStand`) 2 "/Game/Scene/3D/Things/Ski/Map_001.Map_001"))

(event `self.Box.OnComponentEndOverlap`
  (params (OverlappedComponent :type "PrimitiveComponent Object Reference") (OtherActor :type "Actor Object Reference") (OtherComp :type "PrimitiveComponent Object Reference") (OtherBodyIndex :type Integer))
  (bind _asbp_ski_character (cast `/Game/Blueprints/Blueprints/BP_SkiCharacter` OtherActor))
  (set `/Game/Blueprints/Blueprints/BP_SkiCharacter.AtSaveStation` false _asbp_ski_character)
  (`/Game/Blueprints/Blueprints/UI/Hud.EnterPrompt` (`/Game/Blueprints/Blueprints/BP_SkiCharacter.HUD` _asbp_ski_character))
  (`PrimitiveComponent.SetMaterial` (`self.MapStand`) 2 "/Game/Blueprints/Blueprints/3D/Inviz.Inviz"))

(event `/Game/Blueprints/Blueprints/BPI_Chairlift.Use`
  (bind _asbp_ski_character (cast `/Game/Blueprints/Blueprints/BP_SkiCharacter` (`GameplayStatics.GetPlayerCharacter` 0)))
  (`/Game/Blueprints/Blueprints/BP_SkiCharacter.SaveFPgame` _asbp_ski_character))

(fn `UserConstructionScript`)