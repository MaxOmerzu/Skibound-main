(event `DIe`
  (bind _arrowmove (`self.ArrowMove`))
  (bind _deathfreshold (`self.DeathFreshold`))
  (bind _cameraboom (`self.CameraBoom`))
  (set `self.LastRecordedSpeed` (`self.CurrentSpeed`))
  (`KismetSystemLibrary.Delay` (`self.DurationOfDeathCheck`))
  (if (== (`self.CurrentSpeed`) (`self.LastRecordedSpeed`))
    (if (> (`self.CurrentSpeed`) _deathfreshold)
      (`|ExecutionSequence`
        (:`then_0`
          (set `CharacterMovementComponent.MaxFlySpeed` (+ _deathfreshold 300.0) (`self.CharacterMovement`)))
        (:`then_1`
          (`KismetSystemLibrary.Delay` (`KismetMathLibrary.RandomFloatInRange` 0.0 2.0))
          (`self.AddMovementInput` (`SceneComponent.GetUpVector` _arrowmove) 1000.0 true)
          (`self.AddMovementInput` (`SceneComponent.GetForwardVector` _arrowmove) 10000.0 true)
          (`KismetSystemLibrary.Delay` 0.5)
          (`PrimitiveComponent.SetSimulatePhysics` (`self.Mesh`) true)
          (set `SpringArmComponent.CameraLagSpeed` 10.0 _cameraboom)
          (set `SpringArmComponent.CameraRotationLagSpeed` 10.0 _cameraboom)
          (set `CharacterMovementComponent.MaxFlySpeed` 0.0 (`self.CharacterMovement`))
          (`KismetSystemLibrary.Delay` 3.0)
          (`self.SlowDownChecke` :!label _label)))
      (else
        (goto _label)))))

(event `SpeedHAndaling`
  (bind _charactermovement (`self.CharacterMovement`))
  (set `CharacterMovementComponent.MaxFlySpeed` 1100.0 _charactermovement)
  (`KismetSystemLibrary.Delay` 0.03)
  (set `CharacterMovementComponent.MaxFlySpeed` 800.0 _charactermovement))

(event `BORNA mode`
  (bind _charactermovement (`self.CharacterMovement`))
  (bind _deathfreshold (`self.DeathFreshold`))
  (set `self.LastRecordedSpeed_New` (`self.CurrentSpeed`))
  (`KismetSystemLibrary.Delay` 3.0)
  (if (== (`KismetMathLibrary.FTrunc` (`self.LastRecordedSpeed_New`)) (`KismetMathLibrary.FTrunc` (`self.CurrentSpeed`)))
    (set `CharacterMovementComponent.MaxFlySpeed` (+ _deathfreshold 300.0) _charactermovement)
    (else
      (set `CharacterMovementComponent.MaxFlySpeed` _deathfreshold _charactermovement))))

(event `self.ReceiveBeginPlay`
  (bind _asplayer_controller (cast `PlayerController` (`self.GetController`)))
  (bind _returnvalue (pcsubsystem `EnhancedInputLocalPlayerSubsystem` _asplayer_controller))
  (`/Engine/EditorBlueprintResources/StandardMacros.IsValid` _returnvalue
    (:`Is Valid`
      (`EnhancedInputSubsystemInterface.AddMappingContext` _returnvalue "/Game/Blueprints/Input/IMC_Default.IMC_Default" 1 (struct)))))

(event `self.ReceiveTick`
  (params (DeltaSeconds :type "Float (single-precision)"))
  (bind (_relativelocation_x _relativelocation_y) (`KismetMathLibrary.BreakVector` (`SceneComponent.RelativeLocation` (`self.CamArrow`))))
  (`self.CalculateSpeedAndDirection`)
  (`self.SpawnSnowParticles`)
  (`self.SpawnStickSnowParticles` (`self.FX_arrowS`) (`self.sEnd`) (`self.NS_SnowStick1`))
  (`self.SpawnStickSnowParticles` (`self.FX_arrowS2`) (`self.sEnd1`) (`self.NS_SnowStick`))
  (`self.DIe`)
  (`KismetSystemLibrary.PrintString` (`KismetStringLibrary.Conv_DoubleToString` (`self.CurrentSpeed`)) true true (struct :`R` 1.0 :`B` 0.911084 :`A` 1.0) 0.031)
  (`KismetSystemLibrary.PrintString` (`KismetStringLibrary.Conv_DoubleToString` (`CharacterMovementComponent.MaxFlySpeed` (`self.CharacterMovement`))) true true (struct :`R` 1.0 :`G` 0.825801 :`A` 1.0) 0.02)
  (`self.IsInSafeBox`)
  (`SceneComponent.K2_SetRelativeLocation` (`self.Camera`) (`KismetMathLibrary.MakeVector` _relativelocation_x _relativelocation_y 688.0) false false)
  (`SceneComponent.K2_SetWorldRotation` :`self` (`self.Arrow1`))
  (`SceneComponent.K2_SetWorldRotation` :`self` (`self.AngleEnd`))
  (`SceneComponent.K2_SetWorldRotation` :`self` (`self.Angle`))
  (`self.AddMovementInput` (`KismetMathLibrary.NegateVector` (`self.GetActorUpVector`)) 1.0 true)
  (if (== (`SceneComponent.K2_GetComponentRotation` (`self.Arrow1`)) (`SceneComponent.K2_GetComponentRotation` (`self.Arrow2`)) :`ErrorTolerance` 10.0)
    _
    (else
      _))
  (set `CharacterMovementComponent.BrakingDecelerationFlying` 10000.0 (`self.CharacterMovement`))
  (bind _outhit (`KismetSystemLibrary.LineTraceSingle` :`Start` (`SceneComponent.K2_GetComponentLocation` (`self.Angle`)) :`End` (`SceneComponent.K2_GetComponentLocation` (`self.AngleEnd`)) :`TraceChannel` "TraceTypeQuery1" :`DrawTime` 100.0))
  (`KismetSystemLibrary.PrintString` (`KismetStringLibrary.Conv_DoubleToString` 0.0) true true (struct :`G` 1.0 :`B` 0.100954 :`A` 1.0) 0.03)
  (`self.SpeedHAndaling`)
  (`self.BORNA mode`))

(event `EnhancedInput|/Game/Blueprints/Input/Actions/IA_Look`
  (params (ActionValue :type "Vector2D Structure") (ElapsedSeconds :type "Float (double-precision)") (TriggeredSeconds :type "Float (double-precision)") (InputAction :type "InputAction Object Reference" :default "/Game/Blueprints/Input/Actions/IA_Look.IA_Look"))
  (:`Triggered`
    (`self.AddControllerYawInput` ActionValue_X)
    (`self.AddControllerPitchInput` ActionValue_Y)))

(event `EnhancedInput|/Game/Blueprints/Input/Actions/IA_Jump`
  (params (ActionValue :type "Float (double-precision)") (ElapsedSeconds :type "Float (double-precision)") (TriggeredSeconds :type "Float (double-precision)") (InputAction :type "InputAction Object Reference" :default "/Game/Blueprints/Input/Actions/IA_Jump.IA_Jump")))

(event `EnhancedInput|/Game/Blueprints/Input/Actions/IA_Move`
  (params (ActionValue :type "Float (double-precision)") (ElapsedSeconds :type "Float (double-precision)") (TriggeredSeconds :type "Float (double-precision)") (InputAction :type "InputAction Object Reference" :default "/Game/Blueprints/Input/Actions/IA_Move.IA_Move"))
  (bind _returnvalue (`SceneComponent.GetForwardVector` (`self.ArrowMove`)))
  (:`Triggered`
    (if (`self.DisabledMovement`)
      (message `/Game/Blueprints/Blueprints/BPI_Chairlift.Leave` (`self.CurrentChairlift`))
      (elif (`self.Pro?`)
        (if (`self.CanMove`)
          (set `self.CanMove` false)
          (`self.AddMovementInput` _returnvalue ActionValue true)
          (`KismetSystemLibrary.PrintString` (`KismetStringLibrary.Conv_VectorToString` _returnvalue) true true (struct :`R` 1.0 :`G` 0.019892 :`A` 1.0) 0.02)
          (`KismetSystemLibrary.Delay` 0.0)
          (set `self.CanMove` true))))))

(event `EnhancedInput|/Game/Blueprints/Input/Actions/IA_MoveBad`
  (params (ActionValue :type "Float (double-precision)") (ElapsedSeconds :type "Float (double-precision)") (TriggeredSeconds :type "Float (double-precision)") (InputAction :type "InputAction Object Reference" :default "/Game/Blueprints/Input/Actions/IA_MoveBad.IA_MoveBad"))
  (:`Triggered`
    (if (`self.DisabledMovement`)
      (message `/Game/Blueprints/Blueprints/BPI_Chairlift.Leave` (`self.CurrentChairlift`))
      (elif (`self.Pro?`)
        _
        (elif (`self.CanMove`)
          (set `self.CanMove` false)
          (`self.AddMovementInput` (`SceneComponent.GetForwardVector` (`self.ArrowMove`)) ActionValue true)
          (`KismetSystemLibrary.Delay` 0.0)
          (set `self.CanMove` true))))))

(event `Key|Shift+SpaceBar`
  (params (Key :type "Key Structure"))
  (bind _charactermovement (`self.CharacterMovement`))
  (:`Pressed`
    (set `self.Is Stopping` true)
    (`KismetSystemLibrary.DelayUntilNextTick` :!label _label_2)
    (if (`self.Is Stopping`)
      (set `CharacterMovementComponent.MaxFlySpeed` 150.0 _charactermovement)
      (goto _label_2)
      (else
        (set `CharacterMovementComponent.MaxFlySpeed` (`self.DeathFreshold`) _charactermovement)
        (goto _label_2))))
  (:`Released`
    (set `self.Is Stopping` false)))

(event `Key|D`
  (params (Key :type "Key Structure")))

(event `Key|A`
  (params (Key :type "Key Structure")))

(event `Key|T`
  (params (Key :type "Key Structure"))
  (:`Pressed`
    (`/Engine/EditorBlueprintResources/StandardMacros.FlipFlop`
      (:`A`
        (`ActorComponent.Activate` (`self.FP_cam`) false)
        (`ActorComponent.Deactivate` (`self.TP_Cam`)))
      (:`B`
        (`ActorComponent.Activate` (`self.TP_Cam`) false)
        (`ActorComponent.Deactivate` (`self.FP_cam`))))))

(fn `CalculateSpeedAndDirection`
  (bind _returnvalue (`self.GetVelocity`))
  (set `self.CurrentSpeed` (`KismetMathLibrary.VSize` _returnvalue))
  (set `self.Direction` (`KismetAnimationLibrary.CalculateDirection` _returnvalue (`SceneComponent.GetSocketRotation` (`self.ArrowMove`) "None"))))

(fn `IsInSafeBox`
  (if (`self.Pro?`)
    (set `self.PrevPro?` true)
    (else
      (set `self.PrevPro?` false)))
  (if (> (`KismetArrayLibrary.Array_Length` (`PrimitiveComponent.GetOverlappingActors` (`self.Sphere`) "/Game/Blueprints/Misc/SafeBox.SafeBox_C")) 0)
    (`KismetSystemLibrary.PrintString` "in Safe" true true (struct :`G` 0.66 :`B` 1.0 :`A` 1.0) 0.02)
    (set `self.InSafe` true)
    (if (`self.PrevPro?`)
      (set `self.Pro?` false))
    (else
      (`KismetSystemLibrary.PrintString` "Not in Safe" true true (struct :`G` 0.66 :`B` 1.0 :`A` 1.0) 0.02)
      (set `self.InSafe` false))))

(fn `SlowDownChecke`
  (`KismetSystemLibrary.PrintString` (`KismetStringLibrary.Conv_DoubleToString` (`self.Direction`)) true true (struct :`R` 0.957907 :`B` 1.0 :`A` 1.0) 0.02)
  (if (> (`self.CurrentSpeed`) 780.0)
    (set `self.Pro?` true)
    (else
      (set `self.Pro?` false))))

(fn `SpawnSnowParticles`
  (if (> (`self.CurrentSpeed`) 100.0)
    (`SceneComponent.SetHiddenInGame` (`self.NS_SnowSki`) false false)
    (`SceneComponent.SetHiddenInGame` (`self.NS_SnowSki1`) false false)
    (else
      (`SceneComponent.SetHiddenInGame` (`self.NS_SnowSki`) true false)
      (`SceneComponent.SetHiddenInGame` (`self.NS_SnowSki1`) true false))))

(fn `SpawnStickSnowParticles`
  (params (Target :type "SceneComponent Object Reference") (TargetEnd :type "SceneComponent Object Reference") (Particle :type "SceneComponent Object Reference"))
  (bind (_outhit _returnvalue) (`KismetSystemLibrary.LineTraceSingle` :`Start` (`SceneComponent.K2_GetComponentLocation` Target) :`End` (`SceneComponent.K2_GetComponentLocation` TargetEnd) :`TraceChannel` "TraceTypeQuery1" :`DrawTime` 0.5))
  (if _returnvalue
    (`SceneComponent.SetHiddenInGame` Particle false false)
    (else
      (`SceneComponent.SetHiddenInGame` Particle true false))))

(fn `UserConstructionScript`)