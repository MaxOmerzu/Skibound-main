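; ItemGiver is a pickup trigger that unlocks a cosmetic gear item for the ski character that enters it.
; When an actor overlaps its Box, it casts to BP_SkiCharacter and sets the ItemNumber entry true in the unlock array chosen by ItemType.
; Types cover jackets, pants, ski masks, pancerice, helmets and goggles, with types 3 and 4 both writing to UnlockedPancerice.
; The actor stays in place afterward.
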(event `self.Box.OnComponentBeginOverlap`
  (params (OverlappedComponent :type "PrimitiveComponent Object Reference") (OtherActor :type "Actor Object Reference") (OtherComp :type "PrimitiveComponent Object Reference") (OtherBodyIndex :type Integer) (bFromSweep :type Boolean) (SweepResult :type "HitResult Structure (by ref)"))
  (bind _itemnumber (`self.ItemNumber`))
  (bind _asbp_ski_character (cast `/Game/Blueprints/Blueprints/BP_SkiCharacter` OtherActor))
  (if (== (`self.ItemType`) 0)
    (`KismetArrayLibrary.Array_Set` (`/Game/Blueprints/Blueprints/BP_SkiCharacter.UnlockedJackets` _asbp_ski_character) _itemnumber true)
    (elif (== (`self.ItemType`) 1)
      (`KismetArrayLibrary.Array_Set` (`/Game/Blueprints/Blueprints/BP_SkiCharacter.UnlockedPants` _asbp_ski_character) _itemnumber true)
      (elif (== (`self.ItemType`) 2)
        (`KismetArrayLibrary.Array_Set` (`/Game/Blueprints/Blueprints/BP_SkiCharacter.UnlockedSkiMasks` _asbp_ski_character) _itemnumber true)
        (elif (== (`self.ItemType`) 3)
          (bind _unlockedpancerice (`/Game/Blueprints/Blueprints/BP_SkiCharacter.UnlockedPancerice` _asbp_ski_character))
          (`KismetArrayLibrary.Array_Set` _unlockedpancerice _itemnumber true)
          (elif (== (`self.ItemType`) 4)
            (`KismetArrayLibrary.Array_Set` _unlockedpancerice _itemnumber true)
            (elif (== (`self.ItemType`) 5)
              (`KismetArrayLibrary.Array_Set` (`/Game/Blueprints/Blueprints/BP_SkiCharacter.UnlockedHelmets` _asbp_ski_character) _itemnumber true)
              (elif (== (`self.ItemType`) 6)
                (`KismetArrayLibrary.Array_Set` (`/Game/Blueprints/Blueprints/BP_SkiCharacter.UnlockedGoggles` _asbp_ski_character) _itemnumber true)))))))))

(fn `UserConstructionScript`)