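; CustomizationBox is a trigger volume that opens character customization when a BP_SkiCharacter enters it.
; On box overlap, if not already in use, it calls the character's CharacterCreator and marks itself in use.
; It then hands the Arrow component's world location and rotation to the creator (CC) as the exit transform.
; The in-use flag clears when a ski character leaves the box.
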(event `self.Box.OnComponentBeginOverlap`
  (params (OverlappedComponent :type "PrimitiveComponent Object Reference") (OtherActor :type "Actor Object Reference") (OtherComp :type "PrimitiveComponent Object Reference") (OtherBodyIndex :type Integer) (bFromSweep :type Boolean) (SweepResult :type "HitResult Structure (by ref)"))
  (bind _asbp_ski_character (cast `/Game/Blueprints/Blueprints/BP_SkiCharacter` OtherActor))
  (if (not (`self.InUse`))
    (`/Game/Blueprints/Blueprints/BP_SkiCharacter.CharacterCreator` _asbp_ski_character)
    (set `self.InUse` true)
    (bind _cc (`/Game/Blueprints/Blueprints/BP_SkiCharacter.CC` _asbp_ski_character))
    (set `/Game/Blueprints/Blueprints/UI/CharacterCustomiser.ExitLocation` (`SceneComponent.K2_GetComponentLocation` (`self.Arrow`)) _cc)
    (set `/Game/Blueprints/Blueprints/UI/CharacterCustomiser.ExitRotation` (`SceneComponent.K2_GetComponentRotation` (`self.Arrow`)) _cc)))

(event `self.Box.OnComponentEndOverlap`
  (params (OverlappedComponent :type "PrimitiveComponent Object Reference") (OtherActor :type "Actor Object Reference") (OtherComp :type "PrimitiveComponent Object Reference") (OtherBodyIndex :type Integer))
  (cast `/Game/Blueprints/Blueprints/BP_SkiCharacter` OtherActor)
  (set `self.InUse` false))

(fn `UserConstructionScript`)