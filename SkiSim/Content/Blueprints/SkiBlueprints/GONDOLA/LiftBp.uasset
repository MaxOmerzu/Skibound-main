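; LiftBp is a ski lift station that teleports the player's ski character to the lift's end point.
; Its Box overlap sets the character's InQue flag and calls the HUD's EnterPrompt on both entry and exit.
; The EnterChairLift event, not called within this Blueprint, plays a beep, waits briefly, then snaps the character cached at BeginPlay to the EndLocation transform.
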(event `self.ReceiveBeginPlay`
  (bind _asbp_ski_character (cast `/Game/Blueprints/Blueprints/BP_SkiCharacter` (`GameplayStatics.GetPlayerCharacter` 0)))
  (set `self.As BP Ski Character` _asbp_ski_character))

(event `self.Box.OnComponentBeginOverlap`
  (params (OverlappedComponent :type "PrimitiveComponent Object Reference") (OtherActor :type "Actor Object Reference") (OtherComp :type "PrimitiveComponent Object Reference") (OtherBodyIndex :type Integer) (bFromSweep :type Boolean) (SweepResult :type "HitResult Structure (by ref)"))
  (bind _asbp_ski_character (cast `/Game/Blueprints/Blueprints/BP_SkiCharacter` OtherActor))
  (set `/Game/Blueprints/Blueprints/BP_SkiCharacter.InQue` true _asbp_ski_character)
  (`/Game/Blueprints/Blueprints/UI/Hud.EnterPrompt` (`/Game/Blueprints/Blueprints/BP_SkiCharacter.HUD` _asbp_ski_character)))

(event `self.Box.OnComponentEndOverlap`
  (params (OverlappedComponent :type "PrimitiveComponent Object Reference") (OtherActor :type "Actor Object Reference") (OtherComp :type "PrimitiveComponent Object Reference") (OtherBodyIndex :type Integer))
  (bind _asbp_ski_character (cast `/Game/Blueprints/Blueprints/BP_SkiCharacter` OtherActor))
  (set `/Game/Blueprints/Blueprints/BP_SkiCharacter.InQue` false _asbp_ski_character)
  (`/Game/Blueprints/Blueprints/UI/Hud.EnterPrompt` (`/Game/Blueprints/Blueprints/BP_SkiCharacter.HUD` _asbp_ski_character)))

(event `/Game/Blueprints/Blueprints/BPI_Chairlift.EnterChairLift`
  (bind (_returnvalue_location _returnvalue_rotation) (`KismetMathLibrary.BreakTransform` (`SceneComponent.K2_GetComponentToWorld` (`self.EndLocation`))))
  (`GameplayStatics.PlaySound2D` "/Game/Audio/SFX/BeepSoundCue.BeepSoundCue" 1.0 1.0 0.0 null null)
  (`KismetSystemLibrary.Delay` 3.0)
  (`self.K2_SetActorLocationAndRotation` (`self.As BP Ski Character`) _returnvalue_location _returnvalue_rotation false false))

(fn `UserConstructionScript`)